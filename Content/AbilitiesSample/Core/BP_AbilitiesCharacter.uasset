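; Player character for the Abilities sample, with camera-relative movement, mouse look and Gameplay Ability System confirm/cancel input.
; Once init state reaches GameplayReady, it binds CommonHealth to its ability system; becoming view target pushes its GameplayCamera.
; Death start makes the controller ignore move input.
; Death finish queues an authority-only async message carrying event data with PlayerState as instigator and itself as target.
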(event OnDeathStartedEventBP(CommonHealth)
  (params (OwningActor :type Actor%20Object%20Reference))
  (bind _returnvalue (Pawn|GetController))
  (Utilities|IsValid _returnvalue
    (:Is%20Valid
      (Input|SetIgnoreMoveInput _returnvalue true))))

(event OnDeathFinishedEventBP(CommonHealth)
  (params (OwningActor :type Actor%20Object%20Reference))
  (Networking|SwitchHasAuthority
    (:Authority
      (bind _returnvalue (Utilities|InstancedStruct|MakeInstancedStruct (Utilities|Struct|MakeGameplayEventData "(TagName=\"\")" (Variables|Default|GetPlayerState) self)))
      (Class|AsyncMessageSystemBlueprintLibrary|QueueAsyncMessageforBroadcast (Utilities|Struct|MakeAsyncMessageId "(TagName=\"GameplayMessage.Death.Finished\")") _returnvalue))))

(event Input|EnhancedActionEvents|EnhancedInputActionIA_MouseLook
  (params (ActionValue :type Vector%202D%20Structure) (ElapsedSeconds :type Float%20%28double-precision%29) (TriggeredSeconds :type Float%20%28double-precision%29) (InputAction :type Input%20Action%20Object%20Reference :default "/Game/AbilitiesSample/Input/Actions/IA_MouseLook.IA_MouseLook"))
  (bind (_x _y) (Math|Vector2D|BreakVector2D ActionValue))
  (Pawn|Input|AddControllerYawInput _x)
  (Pawn|Input|AddControllerPitchInput _y))

(event Input|EnhancedActionEvents|EnhancedInputActionIA_Move
  (params (ActionValue :type Vector%202D%20Structure) (ElapsedSeconds :type Float%20%28double-precision%29) (TriggeredSeconds :type Float%20%28double-precision%29) (InputAction :type Input%20Action%20Object%20Reference :default "/Game/AbilitiesSample/Input/Actions/IA_Move.IA_Move"))
  (Class|PawnMovementComponent|AddInputVector (Variables|Character|GetCharacterMovement) (Class|KismetMathLibrary|VectorNormal2D (Math|Vector|RotateVector (Math|Conversions|ToVector(Vector2D) ActionValue) (Pawn|GetControlRotation :!class /Script/Engine.Pawn)) 0.0001) false))

(event Input|EnhancedActionEvents|EnhancedInputActionIA_Ability_Confirm
  (params (ActionValue :type Boolean) (ElapsedSeconds :type Float%20%28double-precision%29) (TriggeredSeconds :type Float%20%28double-precision%29) (InputAction :type Input%20Action%20Object%20Reference :default "/Game/AbilitiesSample/Input/Actions/IA_Ability_Confirm.IA_Ability_Confirm"))
  (Class|AbilitySystemComponent|InputConfirm (Ability|GetAbilitySystemComponent 0)))

(event Input|EnhancedActionEvents|EnhancedInputActionIA_Ability_Cancel
  (params (ActionValue :type Boolean) (ElapsedSeconds :type Float%20%28double-precision%29) (TriggeredSeconds :type Float%20%28double-precision%29) (InputAction :type Input%20Action%20Object%20Reference :default "/Game/AbilitiesSample/Input/Actions/IA_Ability_Cancel.IA_Ability_Cancel"))
  (Class|AbilitySystemComponent|InputCancel (Ability|GetAbilitySystemComponent 0)))

(event EventOnBecomeViewTarget
  (params (PC :type Player%20Controller%20Object%20Reference))
  (Class|GameplayCameraComponent|ActivateCameraforPlayerController (Variables|Default|GetGameplayCamera) PC true "Push"))

(event EventBeginPlay
  (|WaitforInitState self "(TagName=\"InitState.GameplayReady\")" true
    (:OnStateReached
      (Class|CommonHealthComponent|SetAbilitySystem (Variables|Default|GetCommonHealth) (Ability|GetAbilitySystemComponent 0)))))

(fn ConstructionScript)