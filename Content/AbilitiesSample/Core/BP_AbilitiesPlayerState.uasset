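; Player state for the abilities sample that relays melee hits, restores health on respawn and supplies UI view models.
; Outgoing damage events tagged as melee go through a multi event that queues a WeaponHit async message.
; When a valid pawn is set on the authority, it applies GE_ResetHealth if the checked attribute is near zero.
; Getters lazily create and cache the activatable-abilities and player-state view models.
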(event Custom|Multi_OnWeaponHit
  (params (Payload :type Gameplay%20Event%20Data%20Structure))
  (bind _returnvalue (Utilities|InstancedStruct|MakeInstancedStruct Payload))
  (Class|AsyncMessageSystemBlueprintLibrary|QueueAsyncMessageforBroadcast (Utilities|Struct|MakeAsyncMessageId "(TagName=\"GameplayMessage.WeaponHit\")") _returnvalue))

(event Custom|OnPawnSet_Event
  (params (Player :type Player%20State%20Object%20Reference) (NewPawn :type Pawn%20Object%20Reference) (OldPawn :type Pawn%20Object%20Reference))
  (Networking|SwitchHasAuthority
    (:Authority
      (Utilities|IsValid NewPawn
        (:Is%20Valid
          (CallFunction|ResetHealth))))))

(event EventBeginPlay
  (EventDispatchers|BindEventtoOnPawnSet (delegate Custom|OnPawnSet_Event))
  (bind _payload (Ability|Async|WaitGameplayEventToActor 0 "(TagName=\"Event.Damage.Outgoing\")" false false)
    (:EventReceived
      (if (GameplayTags|HasAnyTags (Utilities|Struct|BreakGameplayEventData _payload) (GameplayTags|MakeLiteralGameplayTagContainer "(GameplayTags=((TagName=\"Ability.Action.Melee\"),(TagName=\"Ability.Action.Weapon\")))"))
        (CallFunction|MultionWeaponHit _payload)))))

(fn ConstructionScript)

(fn GetActivatableAbilitiesVM
  (bind _vm_activatableabilities (Variables|Default|GetVM_ActivatableAbilities)
    (:then
      (return _vm_activatableabilities))
    (:else
      (bind _returnvalue (Game|ConstructObjectfromClass "/Script/ExtendedGameplayAbilities.VM_ActivatableAbilities"))
      (bind _output_get (Variables|Default|SetVM_ActivatableAbilities _returnvalue))
      (Class|VMActivatableAbilities|SetAbilitySystem _output_get (Class|AbilityPlayerState|GetExtendedAbilitySystemComponent))
      (return (Variables|Default|GetVM_ActivatableAbilities)))))

(fn GetAbilityPlayerStateVM
  (bind _vm_abilityplayerstate (Variables|Default|GetVM_AbilityPlayerState)
    (:then
      (return _vm_abilityplayerstate))
    (:else
      (bind _returnvalue (Game|ConstructObjectfromClass "/Script/ExtendedCommonAbilities.VM_AbilityPlayerState"))
      (bind _output_get (Variables|Default|SetVM_AbilityPlayerState _returnvalue))
      (Class|VMAbilityPlayerState|SetPlayerState _output_get self)
      (return (Variables|Default|GetVM_AbilityPlayerState)))))

(fn ResetHealth
  (bind _returnvalue (Class|AbilityPlayerState|GetExtendedAbilitySystemComponent))
  (if (Math|Float|NearlyEqual(Float) (.ReturnValue (Class|AbilitySystemComponent|GetGameplayAttributeValue _returnvalue "(AttributeName=\"HP\",Attribute=/Script/ExtendedCommonAbilities.HPAttributeSet:HP,AttributeOwner=\"/Script/CoreUObject.Class'/Script/ExtendedCommonAbilities.HPAttributeSet'\")")) 0.0 1e-06)
    (GameplayEffects|ApplyGameplayEffectToSelf :self _returnvalue :GameplayEffectClass "/Game/AbilitiesSample/GameplayEffects/Health/GE_ResetHealth.GE_ResetHealth_C")))