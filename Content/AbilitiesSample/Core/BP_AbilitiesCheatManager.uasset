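; Cheat manager for the abilities sample that provides debug commands to damage the player or change max HP.
; Each command gets the Ability System Component from the player controller's PlayerState.
; HurtSelf and AddMaxHP apply dynamic Gameplay Effects to self, passing the amount through SetByCaller tags.
; HalfHealth reads a float attribute and feeds half its value into HurtSelf.
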(fn HurtSelf
  (params (Amount :type Float%20%28double-precision%29))
  (bind _returnvalue (CallFunction|GetAbilitySystem))
  (bind _returnvalue_2 (Ability|GameplayEffect|AssignTagSetbyCallerMagnitude (GameplayEffects|MakeOutgoingSpec _returnvalue "/Game/AbilitiesSample/GameplayEffects/Damage/GE_Damage_Dynamic.GE_Damage_Dynamic_C" 0.0 (GameplayEffects|MakeEffectContext _returnvalue)) "(TagName=\"Data.Damage\")" Amount))
  (GameplayEffects|ApplyGameplayEffectSpecToSelf _returnvalue _returnvalue_2))

(fn HalfHealth
  (CallFunction|HurtSelf (* (.ReturnValue (Ability|Attribute|GetFloatAttributefromAbilitySystemComponent (CallFunction|GetAbilitySystem) "(AttributeName=\"HP\",Attribute=/Script/ExtendedCommonAbilities.HPAttributeSet:HP,AttributeOwner=\"/Script/CoreUObject.Class'/Script/ExtendedCommonAbilities.HPAttributeSet'\")")) 0.5)))

(fn GetAbilitySystem
  (return (Ability|GetAbilitySystemComponent (Variables|/Script/Engine.Controller|GetPlayerState (Game|GetPlayerController)))))

(fn AddMaxHP
  (params (Amount :type Float%20%28single-precision%29))
  (bind _returnvalue (CallFunction|GetAbilitySystem))
  (bind _returnvalue_2 (Ability|GameplayEffect|AssignTagSetbyCallerMagnitude (GameplayEffects|MakeOutgoingSpec _returnvalue "/Game/AbilitiesSample/GameplayEffects/Health/GE_AddMaxHP_Dynamic.GE_AddMaxHP_Dynamic_C" 0.0 (GameplayEffects|MakeEffectContext _returnvalue)) "(TagName=\"Data.Amount\")" Amount))
  (GameplayEffects|ApplyGameplayEffectSpecToSelf _returnvalue _returnvalue_2))