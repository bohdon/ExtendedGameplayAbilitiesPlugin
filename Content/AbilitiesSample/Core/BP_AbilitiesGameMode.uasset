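; Game mode for the abilities sample that respawns pawns after they die.
; On BeginPlay, with authority only, it listens asynchronously for the Death.Finished gameplay message and reads the dying pawn from the instanced struct payload.
; RespawnPawn destroys that pawn and restarts its controller through RestartPlayer, provided the controller is still valid.
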(event EventBeginPlay
  (Networking|SwitchHasAuthority
    (:Authority
      (bind _message (|StartListeningforAsyncMessage (Utilities|Struct|MakeAsyncMessageId "(TagName=\"GameplayMessage.Death.Finished\")"))
        (:OnMessageReceived
          (bind _value (Utilities|InstancedStruct|GetInstancedStructValue (.PayloadCopy (Utilities|Struct|BreakAsyncMessage _message)))
            (:Valid
              (bind _aspawn (Utilities|Casting|CastToPawn (.Target (Utilities|Struct|BreakGameplayEventData _value))))
              (CallFunction|RespawnPawn _aspawn))))))))

(fn ConstructionScript)

(fn RespawnPawn
  (params (Pawn :type Pawn%20Object%20Reference))
  (bind _returnvalue (Pawn|GetController Pawn))
  (Utilities|IsValid _returnvalue
    (:Is%20Valid
      (Actor|DestroyActor Pawn)
      (Class|GameModeBase|RestartPlayer _returnvalue))))