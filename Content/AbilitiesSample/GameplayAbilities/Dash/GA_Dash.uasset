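; GA_Dash is a gameplay ability that dashes the character in the direction of its last movement input.
; On activation it cancels if there is no input or the commit fails.
; Otherwise it applies a constant-force root motion task along the normalized input vector, using configurable strength and duration.
; Velocity is clamped when the task finishes, and the ability then ends.
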(event Ability|EventActivateAbility
  (bind _output_get (Variables|Default|SetLastInputVector (Pawn|Components|PawnMovement|GetLastInputVector (Variables|/Script/Engine.Character|GetCharacterMovement (Class|ExtendedGameplayAbility|GetCharacterfromActorInfo)))))
  (if (not (Math|Vector|VectorIsNearlyZero _output_get))
    (bind _returnvalue (Ability|CommitAbility))
    (if _returnvalue
      (Ability|Tasks|ApplyRootMotionConstantForce "None" (Math|Vector|Normalize (Variables|Default|GetLastInputVector)) (Variables|Default|GetStrength) (Variables|Default|GetDuration) false 0 "ClampVelocity" "0, 0, 0" 8e+02
        (:OnFinish
          (Ability|EndAbility)))
      (else
        (Ability|CancelAbility)))
    (else
      (Ability|CancelAbility))))