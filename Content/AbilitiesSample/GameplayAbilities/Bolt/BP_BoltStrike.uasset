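; BP_BoltStrike is the area-effect actor for the Bolt ability sample, applying gameplay effects and knockback to actors it hits.
; Construction sizes the collision sphere from Radius and disables collision, which BeginPlay re-enables after a one-second delay.
; Overlapping actors other than the Instigator receive the EffectSpecSet once, tracked through AffectedActors.
; On a successful application, Characters also get a large movement force away from the strike's location.
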(event OnComponentBeginOverlap(EffectCollision)
  (params (OverlappedComponent :type Primitive%20Component%20Object%20Reference) (OtherActor :type Actor%20Object%20Reference) (OtherComp :type Primitive%20Component%20Object%20Reference) (OtherBodyIndex :type Integer) (bFromSweep :type Boolean) (SweepResult :type Hit%20Result%20Structure%20%28by%20ref%29))
  (if (!= OtherActor (Variables|Actor|GetInstigator))
    (bind _bsuccess (Class|ExtendedAbilitySystemStatics|ApplyEffectSpecSettoActorOnce OtherActor (Variables|Default|GetEffectSpecSet) self (Variables|Default|GetAffectedActors)))
    (if _bsuccess
      (bind _ascharacter (Utilities|Casting|CastToCharacter OtherActor))
      (Physics|AddForce (Variables|/Script/Engine.Character|GetCharacterMovement _ascharacter) (* (Math|Vector|Normalize (- (Transformation|GetActorLocation _ascharacter) (Transformation|GetActorLocation))) 5e+06)))))

(event EventBeginPlay
  (Utilities|FlowControl|Delay 1.0)
  (Collision|SetActorEnableCollision true))

(fn ConstructionScript
  (Components|Sphere|SetSphereRadius (Variables|Default|GetEffectCollision) (Variables|Default|GetRadius) false)
  (Collision|SetActorEnableCollision false))