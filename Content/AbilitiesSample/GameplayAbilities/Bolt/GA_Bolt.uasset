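; Gameplay ability for a targeted bolt strike that the player aims with a radius-sized reticle and confirms.
; Activation applies a targeting-state effect to the owner and waits for target data from the GAT_Bolt targeting preset.
; On confirm it commits, clears the targeting effect and spawns BP_BoltStrike with the main effect spec set and radius.
; Cancelling or a failed commit cancels the ability, and ending always removes the targeting effect.
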(event Custom|RemoveTargetingEffect
  (Ability|RemoveGameplayEffectFromOwnerWithHandle (Variables|Default|GetTargetingEffect)))

(event Ability|EventActivateAbility
  (bind _returnvalue (Ability|ApplyGameplayEffectToOwner "/Game/AbilitiesSample/GameplayEffects/Common/GE_State_Targeting.GE_State_Targeting_C"))
  (Variables|Default|SetTargetingEffect _returnvalue)
  (bind _data (|WaitTargetData :ConfirmationType "UserConfirmed" :Class "/Script/ExtendedGameplayAbilities.GameplayAbilityTargetActor_TargetingPreset" :Preset "/Game/AbilitiesSample/GameplayAbilities/Bolt/GAT_Bolt.GAT_Bolt" :ReticleParams (Utilities|Struct|MakeWorldReticleParameters (Math|Conversions|ToVector(Float) (Variables|Default|GetRadius))) :ReticleClass "/Game/AbilitiesSample/GameplayAbilities/Bolt/BP_Bolt_Retcile.BP_Bolt_Retcile_C")
    (:ValidData
      (bind _returnvalue_2 (Ability|CommitAbility))
      (if _returnvalue_2
        (CallFunction|RemoveTargetingEffect)
        (|SpawnActor _data "/Game/AbilitiesSample/GameplayAbilities/Bolt/BP_BoltStrike.BP_BoltStrike_C" (Class|ExtendedGameplayAbility|MakeEffectSpecSetbyTag "(TagName=\"Effect.Set.Main\")") (Variables|Default|GetRadius) (Class|ExtendedGameplayAbility|GetPawnfromActorInfo)
          (:Success
            _)
          (:DidNotSpawn
            _))
        (Ability|EndAbility)
        (else
          (Ability|CancelAbility))))
    (:Cancelled
      (Ability|CancelAbility))))

(event Ability|EventOnEndAbility
  (params (bWasCancelled :type Boolean))
  (CallFunction|RemoveTargetingEffect))