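; Rifle projectile that applies gameplay effects to what it hits and shows impact and tracer FX.
; On the authority, overlaps with non-instigator actors or a movement stop apply an effect spec set once per actor, broadcasting a WeaponHit message on success.
; It then disables collision, halts and sets a short lifespan; where cosmetics run, it snaps to the impact, spawns Niagara FX and deactivates the tracer two ticks later.
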(event OnProjectileStop(ProjectileMovement)
  (params (ImpactResult :type Hit%20Result%20Structure%20%28by%20ref%29))
  (Networking|SwitchHasAuthority
    (:Authority
      (CallFunction|OnHitActor (.HitActor (Collision|BreakHitResult ImpactResult)) ImpactResult))))

(event OnComponentBeginOverlap(Collision)
  (params (OverlappedComponent :type Primitive%20Component%20Object%20Reference) (OtherActor :type Actor%20Object%20Reference) (OtherComp :type Primitive%20Component%20Object%20Reference) (OtherBodyIndex :type Integer) (bFromSweep :type Boolean) (SweepResult :type Hit%20Result%20Structure%20%28by%20ref%29))
  (Networking|SwitchHasAuthority
    (:Authority
      (if (!= OtherActor (Variables|Actor|GetInstigator))
        (CallFunction|OnHitActor OtherActor SweepResult)))))

(event Custom|OnHitActor
  (params (Actor :type Actor%20Object%20Reference) (Hit :type Hit%20Result%20Structure))
  (CallFunction|ApplyHitEffects Actor)
  (CallFunction|StopProjectile Hit))

(event Custom|SendWeaponHitMessage
  (params (EventData :type Gameplay%20Event%20Data%20Structure))
  (Messaging|BroadcastMessage (Subsystems|GetGameplayMessageSubsystem) "(TagName=\"GameplayMessage.WeaponHit\")" EventData))

(event Custom|StopProjectile
  (params (Hit :type Hit%20Result%20Structure))
  (Collision|SetActorEnableCollision false)
  (Components|Movement|StopMovementImmediately (Variables|Default|GetProjectileMovement))
  (Actor|SetLifeSpan 2.0)
  (Networking|CanExecuteCosmeticEvents
    (:True
      (Transformation|SetActorLocation (.Location (Collision|BreakHitResult Hit)) false false)
      (CallFunction|SpawnImpactFX Hit)
      (Utilities|FlowControl|DelayUntilNextTick)
      (Utilities|FlowControl|DelayUntilNextTick)
      (Components|Activation|Deactivate (Variables|Default|GetFX_Tracer)))))

(fn ConstructionScript
  (Variables|/Script/Engine.ProjectileMovementComponent|SetInitialSpeed (Variables|Default|GetProjectileMovement) (* (Variables|Default|GetSpeed) 1e+02)))

(fn ApplyHitEffects
  (params (Actor :type Actor%20Object%20Reference))
  (bind _returnvalue (Transformation|GetActorLocation))
  (Networking|SwitchHasAuthority
    (:Authority
      (bind _bsuccess (Class|ExtendedAbilitySystemStatics|ApplyEffectSpecSettoActorOnce Actor (Variables|Default|GetEffectSpecSet) self (Variables|Default|GetAffectedActors)))
      (if _bsuccess
        (CallFunction|SendWeaponHitMessage (Utilities|Struct|MakeGameplayEventData "(TagName=\"\")" (Variables|Actor|GetInstigator) 0 0 0 "()" "(GameplayTags=)" "(GameplayTags=)" 0.0 (Ability|TargetData|AbilityTargetDatafromHitResult (Collision|MakeHitResult false false 0.0 0.0 _returnvalue _returnvalue "0,0,1" "0,0,1" 0 Actor))))))))

(fn SpawnImpactFX
  (params (Hit :type Hit%20Result%20Structure))
  (bind (_bblockinghit _binitialoverlap _time _distance _location _impactpoint _normal) (Collision|BreakHitResult Hit))
  (Niagara|SpawnSystematLocation "/Game/AbilitiesSample/GameplayAbilities/Rifle/FX/NS_Rifle_Projectile_Impact.NS_Rifle_Projectile_Impact" _impactpoint (Math|Rotator|MakeRotfromX _normal)))