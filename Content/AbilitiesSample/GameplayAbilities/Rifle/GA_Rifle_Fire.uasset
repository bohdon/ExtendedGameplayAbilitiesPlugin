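; Gameplay ability for automatic rifle fire, repeating at FireRate while input is held and ending on release.
; Each shot commits the ability, checks blocking tags, then gets an instant aim point from a targeting preset.
; It spawns a projectile from the eye point, carrying an effect set with DPS/FireRate damage as set-by-caller magnitude.
; Random cone spread widens over the first three seconds; failed or blocked shots retry next interval.
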(event Custom|ScheduleNextFire
  (Ability|Tasks|WaitDelay (/ 1.0 (Variables|Default|GetFireRate))
    (:OnFinish
      (CallFunction|Fire))))

(event Custom|Fire
  (bind _returnvalue (Ability|CommitAbility))
  (if _returnvalue
    (if (not (GameplayTags|HasAnyMatchingGameplayTags (Ability|GetAbilitySystemComponentfromActorInfo) (Variables|Default|GetBlockFiringTags)))
      (bind _data (|WaitTargetData :ConfirmationType "Instant" :Class "/Script/ExtendedGameplayAbilities.GameplayAbilityTargetActor_TargetingPreset" :Preset "/Game/AbilitiesSample/GameplayAbilities/Rifle/GAT_Rifle_Fire.GAT_Rifle_Fire" :ReticleClass 0)
        (:ValidData
          (CallFunction|FireatLocation (.Location (Collision|BreakHitResult (Ability|TargetData|GetHitResultfromTargetData _data))))))
      (else
        (CallFunction|ScheduleNextFire)))
    (else
      (CallFunction|ScheduleNextFire))))

(event Custom|FireAtLocation
  (params (TargetLocation :type Vector))
  (bind _returnvalue (CallFunction|GetProjectileTargetData TargetLocation))
  (bind _returnvalue_2 (Class|ExtendedAbilitySystemStatics|AssignTagSetbyCallerMagnitudeforSet (Class|ExtendedGameplayAbility|MakeEffectSpecSetbyTag "(TagName=\"Effect.Set.Main\")") "(TagName=\"Data.Damage\")" (/ (Variables|Default|GetDPS) (Variables|Default|GetFireRate))))
  (|SpawnActor _returnvalue "/Game/AbilitiesSample/GameplayAbilities/Rifle/BP_Rifle_Projectile.BP_Rifle_Projectile_C" _returnvalue_2 (Variables|Default|GetSpeed) (Class|ExtendedGameplayAbility|GetPawnfromActorInfo)
    (:then
      (CallFunction|ScheduleNextFire))))

(event Ability|EventActivateAbility
  (Ability|Tasks|WaitInputRelease true
    (:then
      (Variables|Default|SetActivateTime (Utilities|Time|GetTimeSeconds))
      (CallFunction|Fire))
    (:OnRelease
      (Ability|EndAbility))))

(fn GetProjectileTargetData
  (params (TargetLocation :type Vector))
  (bind _returnvalue (Class|ExtendedGameplayAbility|GetCharacterfromActorInfo))
  (bind _returnvalue_2 (Utilities|Time|GetTimeSeconds))
  (bind _spreadhalfangle (Variables|Default|GetSpreadHalfAngle))
  (bind _activatetime (Variables|Default|GetActivateTime))
  (bind _outlocation (Actor|GetActorEyesViewPoint _returnvalue))
  (bind _returnvalue_3 (- _returnvalue_2 _activatetime))
  (bind _returnvalue_4 (Math|Float|MapRangeClamped _returnvalue_3 0.0 3.0 0.0 1.0))
  (bind _returnvalue_5 (- TargetLocation _outlocation))
  (bind _returnvalue_6 (* _spreadhalfangle _returnvalue_4))
  (bind _returnvalue_7 (Math|Random|RandomUnitVectorinConeinDegrees _returnvalue_5 _returnvalue_6))
  (bind _returnvalue_8 (Math|Rotator|MakeRotfromX _returnvalue_7))
  (bind _returnvalue_9 (Math|Transform|MakeTransform _outlocation _returnvalue_8))
  (bind _gameplayabilitytargetinglocationinfo (Utilities|Struct|MakeGameplayAbilityTargetingLocationInfo 0 0 0 _returnvalue_9))
  (return (Class|AbilitySystemBlueprintLibrary|AbilityTargetDatafromLocations _gameplayabilitytargetinglocationinfo _gameplayabilitytargetinglocationinfo)))