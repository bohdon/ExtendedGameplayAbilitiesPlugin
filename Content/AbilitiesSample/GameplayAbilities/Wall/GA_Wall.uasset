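; Gameplay ability that lets the player target, rotate and spawn a temporary BP_Wall.
; User-confirmed targeting uses the GAT_Wall preset, a reticle and a temporary input context for rotation, sending yaw to the server and exposing it relative to the avatar.
; On confirm it commits and spawns the wall for its Duration; another input press cancels early.
; Ending the ability hides and destroys the spawned wall.
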(event Custom|ServerSetTargetingRotation
  (params (YawRotation :type Float%20%28double-precision%29))
  (Variables|Default|SetTargetingRotation (Math|Rotator|MakeRotator 0.0 0.0 YawRotation)))

(event Input|EnhancedActionEvents|EnhancedInputActionIA_Ability_Wall_Rotate
  (params (ActionValue :type Float%20%28double-precision%29) (ElapsedSeconds :type Float%20%28double-precision%29) (TriggeredSeconds :type Float%20%28double-precision%29) (InputAction :type Input%20Action%20Object%20Reference :default "/Game/AbilitiesSample/GameplayAbilities/Wall/Input/IA_Ability_Wall_Rotate.IA_Ability_Wall_Rotate"))
  (bind _output_get (Variables|Default|SetTargetingRotation (Math|Rotator|CombineRotators (Math|Rotator|MakeRotator 0.0 0.0 ActionValue) (Variables|Default|GetTargetingRotation))))
  (CallFunction|ServerSetTargetingRotation (.Yaw (Math|Rotator|BreakRotator _output_get))))

(event Ability|EventActivateAbility
  (bind _size (Variables|Default|GetSize))
  (CallFunction|StartTargeting)
  (Class|ExtendedGameplayAbility|AddInputMappingContext "/Game/AbilitiesSample/GameplayAbilities/Wall/Input/IMC_Ability_Wall.IMC_Ability_Wall" 0 (Utilities|Struct|MakeModifyContextOptions false false false))
  (Variables|Default|SetTargetingRotation "0, 0, 0")
  (bind _data (|WaitTargetData :TaskInstanceName "Targeting" :ConfirmationType "UserConfirmed" :Class "/Script/ExtendedGameplayAbilities.GameplayAbilityTargetActor_TargetingPreset" :Preset "/Game/AbilitiesSample/GameplayAbilities/Wall/GAT_Wall.GAT_Wall" :ReticleParams (Utilities|Struct|MakeWorldReticleParameters (Math|Vector|MakeVector (Utilities|GetClassDefaults "/Game/AbilitiesSample/GameplayAbilities/Wall/BP_Wall.BP_Wall_C") (.x _size) (.y _size))) :ReticleClass "/Game/AbilitiesSample/GameplayAbilities/Wall/BP_Wall_Reticle.BP_Wall_Reticle_C")
    (:ValidData
      (CallFunction|EndTargeting)
      (bind _returnvalue (Ability|CommitAbility))
      (if _returnvalue
        (bind _spawnedactor (|SpawnActor _data "/Game/AbilitiesSample/GameplayAbilities/Wall/BP_Wall.BP_Wall_C" (Variables|Default|GetDuration) (Variables|Default|GetSize) (Class|ExtendedGameplayAbility|GetPawnfromActorInfo))
          (:then
            (Ability|Tasks|WaitDelay (Variables|Default|GetDuration)
              (:then
                (Ability|Tasks|WaitInputPress false
                  (:OnPress
                    (Ability|CancelAbility))))
              (:OnFinish
                (Ability|EndAbility))))
          (:Success
            (bind _asbp_wall (Utilities|Casting|CastToBP_Wall _spawnedactor))
            (Variables|Default|SetSpawnedWall _asbp_wall)))
        (else
          (Ability|CancelAbility))))
    (:Cancelled
      (Ability|CancelAbility))))

(event EventEndTargeting
  (|CallParentFunction)
  (Class|ExtendedGameplayAbility|RemoveInputMappingContext "/Game/AbilitiesSample/GameplayAbilities/Wall/Input/IMC_Ability_Wall.IMC_Ability_Wall" (Utilities|Struct|MakeModifyContextOptions false false false)))

(event Ability|EventOnEndAbility
  (params (bWasCancelled :type Boolean))
  (|CallParentFunction bWasCancelled)
  (bind _spawnedwall (Variables|Default|GetSpawnedWall)
    (:then
      (Default|HideandDestroy _spawnedwall))
    (:else)))

(fn GetWallRotation
  (return (Math|Rotator|CombineRotators (Variables|Default|GetTargetingRotation) (Transformation|GetActorRotation (Ability|GetAvatarActorfromActorInfo)))))