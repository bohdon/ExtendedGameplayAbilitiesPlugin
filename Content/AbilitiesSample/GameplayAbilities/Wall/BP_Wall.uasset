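; BP_Wall is a temporary wall actor for the Wall sample ability, removed after a set Duration.
; Its construction script scales and raises the cube mesh from Size and WallThickness.
; On BeginPlay it starts the expiry timer and, where cosmetics can run, a timeline meant to fade the material's Alpha over FadeInDuration.
; On expiry it disables collision, reverses that timeline and sets its lifespan to the fade duration.
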(event Custom|HideAndDestroy
  (Utilities|Time|ClearandInvalidateTimerbyHandle (Variables|Default|GetDurationTimer))
  (Collision|SetActorEnableCollision false)
  (Actor|SetLifeSpan (Variables|Default|GetFadeInDuration))
  (CallFunction|Hide))

(event Custom|Hide
  (Networking|CanExecuteCosmeticEvents
    (:True
      (Utilities|String|Reverse (Variables|Default|GetFadeIn_Timeline)))))

(event EventBeginPlay
  (bind _fadein_timeline (Variables|Default|GetFadeIn_Timeline))
  (bind _returnvalue (Utilities|Time|SetTimerbyEvent (delegate Custom|HideAndDestroy) (Variables|Default|GetDuration)))
  (Variables|Default|SetDurationTimer _returnvalue)
  (Networking|CanExecuteCosmeticEvents
    (:True
      (Rendering|Material|SetScalarParameterValueonMaterials (Variables|Default|GetCubeMesh) "Alpha" 0.0)
      (Components|Timeline|PlayfromStart _fadein_timeline)
      (Components|Timeline|SetPlayRate _fadein_timeline (/ 1.0 (Variables|Default|GetFadeInDuration))))))

(fn ConstructionScript
  (bind _cubemesh (Variables|Default|GetCubeMesh))
  (bind _size (Variables|Default|GetSize))
  (bind _wallthickness (Variables|Default|GetWallThickness))
  (bind _returnvalue (Math|Vector|MakeVector _wallthickness (.x _size) (.y _size)))
  (Transformation|SetRelativeScale3D _cubemesh (/ _returnvalue 5e+01))
  (Transformation|SetRelativeLocation _cubemesh (Math|Vector|MakeVector 0.0 0.0 (/ (.Z (Math|Vector|BreakVector _returnvalue)) 1.0)) false false))