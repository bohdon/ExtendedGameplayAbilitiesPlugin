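; Targeting trace task for the Teleport ability that supplies the size and length of its trace.
; It overrides the swept radius and half height with the scaled capsule of the instigating Character, taken from the targeting source context.
; Trace length comes from the Range class default on GA_Teleport, so the targeting distance follows the ability's setting.
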(fn GetSweptTraceRadius
  (params (TargetingHandle :type Targeting%20Request%20Handle%20Structure%20%28by%20ref%29))
  (bind _returnvalue (CallFunction|GetCharacter TargetingHandle))
  (Utilities|IsValid _returnvalue
    (:Is%20Valid
      (return (Components|Capsule|GetScaledCapsuleRadius (Variables|/Script/Engine.Character|GetCapsuleComponent _returnvalue))))))

(fn GetSweptTraceCapsuleHalfHeight
  (params (TargetingHandle :type Targeting%20Request%20Handle%20Structure%20%28by%20ref%29))
  (bind _returnvalue (CallFunction|GetCharacter TargetingHandle))
  (Utilities|IsValid _returnvalue
    (:Is%20Valid
      (return (Components|Capsule|GetScaledCapsuleHalfHeight (Variables|/Script/Engine.Character|GetCapsuleComponent _returnvalue))))))

(fn GetTraceLength
  (params (TargetingHandle :type Targeting%20Request%20Handle%20Structure%20%28by%20ref%29))
  (return (.Range (Utilities|GetClassDefaults "/Game/AbilitiesSample/GameplayAbilities/Teleport/GA_Teleport.GA_Teleport_C"))))

(fn GetCharacter
  (params (TargetingHandle :type Targeting%20Request%20Handle%20Structure%20%28by%20ref%29))
  (bind _ascharacter (Utilities|Casting|CastToCharacter (.InstigatorActor (Utilities|Struct|BreakTargetingSourceContext (Class|TargetingSubsystem|GetTargetingSourceContext (Class|TargetingTask|GetTargetingSubsystem TargetingHandle) TargetingHandle)))))
  (return _ascharacter))