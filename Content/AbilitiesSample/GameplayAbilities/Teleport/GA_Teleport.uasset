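; GA_Teleport is a gameplay ability that moves the avatar a set range along the controller's aim, acting as a short dash-style teleport.
; On activation it commits the ability, waits for a cast time, then applies a root motion move-to force toward that point over a fraction of a second.
; Exit velocity is clamped, and the ability ends when the motion times out, whether or not the destination is reached.
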(event Ability|EventActivateAbility
  (bind _returnvalue (Ability|CommitAbility))
  (if _returnvalue
    (Ability|Tasks|WaitDelay (Variables|Default|GetCastTime)
      (:OnFinish
        (Ability|Tasks|ApplyRootMotionMoveToForce "None" (+ (Transformation|GetActorLocation (Ability|GetAvatarActorfromActorInfo)) (* (Math|Vector|GetForwardVector (Pawn|GetControlRotation (Class|ExtendedGameplayAbility|GetPawnfromActorInfo) :!class /Script/Engine.Pawn)) (Variables|Default|GetRange))) 0.1 false "MOVE_None" false 0 "ClampVelocity" "0, 0, 0" 5e+02
          (:OnTimedOut
            _)
          (:OnTimedOutAndDestinationReached
            _))
        (Ability|EndAbility)))))