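; Healing aura volume actor that follows its Instigator and applies a gameplay effect spec set to actors inside it.
; On BeginPlay it snaps and attaches to the Instigator; the construction script sizes the collision sphere from Radius.
; Overlap begin applies the effects once per actor, tracked in AffectedActors, and overlap end removes them using the volume as source object.
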(event OnComponentBeginOverlap(VolumeCollision)
  (params (OverlappedComponent :type Primitive%20Component%20Object%20Reference) (OtherActor :type Actor%20Object%20Reference) (OtherComp :type Primitive%20Component%20Object%20Reference) (OtherBodyIndex :type Integer) (bFromSweep :type Boolean) (SweepResult :type Hit%20Result%20Structure%20%28by%20ref%29))
  (Class|ExtendedAbilitySystemStatics|ApplyEffectSpecSettoActorOnce OtherActor (Variables|Default|GetEffectSpecSet) self (Variables|Default|GetAffectedActors)))

(event OnComponentEndOverlap(VolumeCollision)
  (params (OverlappedComponent :type Primitive%20Component%20Object%20Reference) (OtherActor :type Actor%20Object%20Reference) (OtherComp :type Primitive%20Component%20Object%20Reference) (OtherBodyIndex :type Integer))
  (Class|ExtendedAbilitySystemStatics|RemoveEffectsfromActorbySourceObject OtherActor self (Variables|Default|GetAffectedActors)))

(event EventBeginPlay
  (bind _instigator (Variables|Actor|GetInstigator)
    (:then
      (Transformation|AttachActorToActor _instigator "None" "SnapToTarget" "SnapToTarget" "SnapToTarget" true))
    (:else)))

(fn ConstructionScript
  (Components|Sphere|SetSphereRadius (Variables|Default|GetVolumeCollision) (Variables|Default|GetRadius) true))