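; GA_HealingAura is a gameplay ability that creates a timed healing aura by spawning a BP_HealingAuraVolume, using the avatar actor as target data.
; After committing, it passes radius, duration, instigator pawn and the main effect spec set to the volume through a SpawnActor task.
; The ability ends after the duration, cancels if commit or spawn fails, and destroys any spawned volume when it ends.
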(event Ability|EventActivateAbility
  (bind _returnvalue (Ability|CommitAbility))
  (if _returnvalue
    (bind _spawnedactor (|SpawnActor (Ability|TargetData|AbilityTargetDatafromActor (Ability|GetAvatarActorfromActorInfo)) "/Game/AbilitiesSample/GameplayAbilities/HealingAura/BP_HealingAuraVolume.BP_HealingAuraVolume_C" (Variables|Default|GetRadius) (Variables|Default|GetDuration) (Class|ExtendedGameplayAbility|MakeEffectSpecSetbyTag "(TagName=\"Effect.Set.Main\")") (Class|ExtendedGameplayAbility|GetPawnfromActorInfo))
      (:Success
        (Variables|Default|SetVolumeActor _spawnedactor)
        (Ability|Tasks|WaitDelay (Variables|Default|GetDuration)
          (:OnFinish
            (Ability|EndAbility))))
      (:DidNotSpawn
        (Ability|CancelAbility)))
    (else
      (Ability|CancelAbility))))

(event Ability|EventOnEndAbility
  (params (bWasCancelled :type Boolean))
  (bind _volumeactor (Variables|Default|GetVolumeActor)
    (:then
      (Actor|DestroyActor _volumeactor)
      (Variables|Default|SetVolumeActor 0))
    (:else)))