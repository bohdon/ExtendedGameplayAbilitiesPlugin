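; Base gameplay ability that gives targeted abilities a shared "Targeting" phase, opened by StartTargeting and closed by EndTargeting.
; The phase runs as an ability state that applies the GE_State_Targeting effect and state tag, then removes both when it ends or is interrupted.
; An optional flag cancels other abilities in the targeting state through the ExtendedAbilitySystemComponent, sparing this one.
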(event Custom|StartTargeting
  (|StartAbilityState "Targeting" true
    (:then
      (bind _returnvalue (Ability|ApplyGameplayEffectToOwner "/Game/AbilitiesSample/GameplayEffects/Common/GE_State_Targeting.GE_State_Targeting_C"))
      (Variables|Targeting|SetTargetingStateEffect _returnvalue)
      (Class|ExtendedGameplayAbility|AddAbilityStateTag "(TagName=\"Ability.State.Targeting\")")
      (if (Variables|Targeting|GetCancelOtherTargetingAbilities)
        (bind _asextended_ability_system_component (Utilities|Casting|CastToExtendedAbilitySystemComponent (Ability|GetAbilitySystemComponentfromActorInfo)))
        (Class|ExtendedAbilitySystemComponent|CancelAbilitieswithState _asextended_ability_system_component "(GameplayTags=((TagName=\"Ability.State.Targeting\")))" self)))
    (:OnStateEnded
      (Ability|RemoveGameplayEffectFromOwnerWithHandle (Variables|Targeting|GetTargetingStateEffect) :!label _label)
      (Class|ExtendedGameplayAbility|RemoveAbilityStateTag "(TagName=\"Ability.State.Targeting\")"))
    (:OnStateInterrupted
      (goto _label))))

(event Custom|EndTargeting
  (Class|GameplayAbility|EndAbilityState "Targeting"))