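; BP_SampleVolumeBase is a trigger volume base in the AbilitiesSample, with a box collision and a colored floor mesh.
; Its construction script applies the Size property to the box's X and Y extents, keeps its Z extent, and raises the box to rest on its relative origin.
; It then scales the floor mesh to the box footprint and sets its BaseColor material parameter from the Color property.
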(fn ConstructionScript
  (bind _volumecollision (Variables|Default|GetVolumeCollision))
  (bind _floormesh (Variables|Default|GetFloorMesh))
  (bind _volumecollision_2 (Variables|Default|GetVolumeCollision))
  (bind _size (Variables|Volume|GetSize))
  (bind _returnvalue (Components|Box|GetScaledBoxExtent _volumecollision))
  (bind _returnvalue_2 (* _returnvalue 0.02))
  (bind (_x _y) (Math|Vector|BreakVector _returnvalue_2))
  (Components|Box|SetBoxExtent _volumecollision_2 (Math|Vector|MakeVector (.x _size) (.y _size) (.z (Variables|/Script/Engine.BoxComponent|GetBoxExtent _volumecollision_2))) true)
  (Transformation|SetRelativeLocation _volumecollision_2 (Math|Vector|MakeVector 0.0 0.0 (.z (Components|Box|GetScaledBoxExtent _volumecollision_2))) false false)
  (Transformation|SetRelativeScale3D _floormesh (Math|Vector|MakeVector _x _y (.z (Variables|/Script/Engine.SceneComponent|GetRelativeScale3D _floormesh))))
  (Rendering|Material|SetVectorParameterValueonMaterials (Variables|Default|GetFloorMesh) "BaseColor" (Math|Conversions|ToVector(LinearColor) (Variables|Volume|GetColor))))