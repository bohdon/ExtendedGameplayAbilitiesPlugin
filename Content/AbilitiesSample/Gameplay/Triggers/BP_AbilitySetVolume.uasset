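; BP_AbilitySetVolume is a trigger volume that temporarily grants a GAS ability set to actors inside it.
; On begin overlap it gives the configured set to the actor's Ability System Component, with itself as source object.
; The returned handles are stored in a map keyed by component, preventing duplicate grants.
; On end overlap those handles remove the set, including its attribute sets, and the map entry is cleared.
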(event OnComponentBeginOverlap(VolumeCollision)
  (params (OverlappedComponent :type Primitive%20Component%20Object%20Reference) (OtherActor :type Actor%20Object%20Reference) (OtherComp :type Primitive%20Component%20Object%20Reference) (OtherBodyIndex :type Integer) (bFromSweep :type Boolean) (SweepResult :type Hit%20Result%20Structure%20%28by%20ref%29))
  (CallFunction|GiveAbilitySettoActor OtherActor))

(event OnComponentEndOverlap(VolumeCollision)
  (params (OverlappedComponent :type Primitive%20Component%20Object%20Reference) (OtherActor :type Actor%20Object%20Reference) (OtherComp :type Primitive%20Component%20Object%20Reference) (OtherBodyIndex :type Integer))
  (CallFunction|RemoveAbilitySetfromActor OtherActor))

(fn ConstructionScript
  (|CallParentFunction))

(fn GiveAbilitySettoActor
  (params (Actor :type Actor%20Object%20Reference))
  (bind _output_get (LocalVariables|SetAbilitySystem (Ability|GetAbilitySystemComponent Actor)))
  (Utilities|IsValid _output_get
    (:Is%20Valid
      (if (not (Utilities|Map|Contains (Variables|Default|GetGrantedAbilitySets) (LocalVariables|GetAbilitySystem)))
        (bind _returnvalue (Class|ExtendedAbilitySystemStatics|GiveAbilitySet (LocalVariables|GetAbilitySystem) (Variables|Abilities|GetAbilitySet) self -1))
        (Utilities|Map|Add (Variables|Default|GetGrantedAbilitySets) (LocalVariables|GetAbilitySystem) _returnvalue)))))

(fn RemoveAbilitySetfromActor
  (params (Actor :type Actor%20Object%20Reference))
  (bind _grantedabilitysets (Variables|Default|GetGrantedAbilitySets))
  (bind _output_get (LocalVariables|SetAbilitySystem (Ability|GetAbilitySystemComponent Actor)))
  (Utilities|IsValid _output_get
    (:Is%20Valid
      (if (Utilities|Map|Contains _grantedabilitysets (LocalVariables|GetAbilitySystem))
        (Class|ExtendedAbilitySystemStatics|RemoveAbilitySet (LocalVariables|GetAbilitySystem) (.Value (Utilities|Map|Find _grantedabilitysets (LocalVariables|GetAbilitySystem))) false)
        (Utilities|Map|Remove (Variables|Default|GetGrantedAbilitySets) (LocalVariables|GetAbilitySystem))))))