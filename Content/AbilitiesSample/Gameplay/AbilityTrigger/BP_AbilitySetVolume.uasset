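; BP_AbilitySetVolume is a trigger volume that temporarily grants a Gameplay Ability System ability set to actors standing inside it.
; On begin overlap it gives the set to the actor's ability system component and stores the returned handles in a map keyed by component, preventing duplicate grants.
; End overlap removes the set, including its attribute sets.
; The construction script sizes the box from Size and fits the floor mesh beneath it.
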(event OnComponentBeginOverlap(VolumeCollision)
  (params (OverlappedComponent :type Primitive%20Component%20Object%20Reference) (OtherActor :type Actor%20Object%20Reference) (OtherComp :type Primitive%20Component%20Object%20Reference) (OtherBodyIndex :type Integer) (bFromSweep :type Boolean) (SweepResult :type Hit%20Result%20Structure%20%28by%20ref%29))
  (CallFunction|GiveAbilitySettoActor OtherActor))

(event OnComponentEndOverlap(VolumeCollision)
  (params (OverlappedComponent :type Primitive%20Component%20Object%20Reference) (OtherActor :type Actor%20Object%20Reference) (OtherComp :type Primitive%20Component%20Object%20Reference) (OtherBodyIndex :type Integer))
  (CallFunction|RemoveAbilitySetfromActor OtherActor))

(fn ConstructionScript
  (bind _volumecollision (Variables|Default|GetVolumeCollision))
  (bind _floormesh (Variables|Default|GetFloorMesh))
  (bind _volumecollision_2 (Variables|Default|GetVolumeCollision))
  (bind _size (Variables|Default|GetSize))
  (bind _returnvalue (Components|Box|GetScaledBoxExtent _volumecollision))
  (bind _returnvalue_2 (* _returnvalue 0.02))
  (bind (_x _y) (Math|Vector|BreakVector _returnvalue_2))
  (Components|Box|SetBoxExtent _volumecollision_2 (Math|Vector|MakeVector (.x _size) (.y _size) (.z (Variables|/Script/Engine.BoxComponent|GetBoxExtent _volumecollision_2))) true)
  (Transformation|SetRelativeLocation _volumecollision_2 (Math|Vector|MakeVector 0.0 0.0 (.z (Components|Box|GetScaledBoxExtent _volumecollision_2))) false false)
  (Transformation|SetRelativeScale3D _floormesh (Math|Vector|MakeVector _x _y (.z (Variables|/Script/Engine.SceneComponent|GetRelativeScale3D _floormesh)))))

(fn GiveAbilitySettoActor
  (params (Actor :type Actor%20Object%20Reference))
  (bind _output_get (LocalVariables|SetAbilitySystem (Ability|GetAbilitySystemComponent Actor)))
  (Utilities|IsValid _output_get
    (:Is%20Valid
      (if (not (Utilities|Map|Contains (Variables|Default|GetGrantedAbilitySets) (LocalVariables|GetAbilitySystem)))
        (bind _returnvalue (Class|ExtendedAbilitySystemStatics|GiveAbilitySet (LocalVariables|GetAbilitySystem) (Variables|Default|GetAbilitySet) self -1))
        (Utilities|Map|Add (Variables|Default|GetGrantedAbilitySets) (LocalVariables|GetAbilitySystem) _returnvalue)))))

(fn RemoveAbilitySetfromActor
  (params (Actor :type Actor%20Object%20Reference))
  (bind _grantedabilitysets (Variables|Default|GetGrantedAbilitySets))
  (bind _output_get (LocalVariables|SetAbilitySystem (Ability|GetAbilitySystemComponent Actor)))
  (Utilities|IsValid _output_get
    (:Is%20Valid
      (if (Utilities|Map|Contains _grantedabilitysets (LocalVariables|GetAbilitySystem))
        (Class|ExtendedAbilitySystemStatics|RemoveAbilitySet (LocalVariables|GetAbilitySystem) (.Value (Utilities|Map|Find _grantedabilitysets (LocalVariables|GetAbilitySystem))) false)
        (Utilities|Map|Remove (Variables|Default|GetGrantedAbilitySets) (LocalVariables|GetAbilitySystem))))))